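; Weapon pickup actor that arms or resupplies a VehicleBlueprint overlapping it.
; On overlap it compares WeaponClass to the vehicle's primary and secondary weapons, adding that weapon's InitialAmmo on a match.
; Otherwise it spawns the weapon onto the free GunMount or SecondGunMount socket, or prints that slots are full.
; The pickup never destroys itself; Tick is empty and the bobbing movement logic is unconnected.
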(event `self.ReceiveActorBeginOverlap`
  (params (OtherActor :type "Actor Object Reference"))
  (bind _weaponclass (`self.WeaponClass`))
  ;[1 1 1] Weapon Pickup
  (bind _asvehicle_blueprint (cast `/Game/VehicleAdvBP/Blueprints/VehicleBlueprint` OtherActor))
  (bind _currentweapon (`/Game/VehicleAdvBP/Blueprints/VehicleBlueprint.CurrentWeapon` _asvehicle_blueprint))
  (if (`KismetSystemLibrary.IsValid` _currentweapon)
    (if (== _weaponclass (`GameplayStatics.GetObjectClass` _currentweapon))
      (set `/Game/VehicleAdvBP/Blueprints/BP_BaseWeapon.CurrentAmmo` (+ (`/Game/VehicleAdvBP/Blueprints/BP_BaseWeapon.CurrentAmmo` _currentweapon) (`/Game/VehicleAdvBP/Blueprints/BP_BaseWeapon.InitialAmmo` _currentweapon)) _currentweapon)
      (else
        (bind _secondaryweapon (`/Game/VehicleAdvBP/Blueprints/VehicleBlueprint.SecondaryWeapon` _asvehicle_blueprint))
        (if (`KismetSystemLibrary.IsValid` _secondaryweapon)
          (if (== (`GameplayStatics.GetObjectClass` _secondaryweapon) _weaponclass)
            (bind _returnvalue (+ (`/Game/VehicleAdvBP/Blueprints/BP_BaseWeapon.CurrentAmmo` _secondaryweapon) (`/Game/VehicleAdvBP/Blueprints/BP_BaseWeapon.InitialAmmo` _secondaryweapon)))
            (set `/Game/VehicleAdvBP/Blueprints/BP_BaseWeapon.CurrentAmmo` _returnvalue _secondaryweapon)
            (else
              (`KismetSystemLibrary.PrintString` "No weapon slots available")))
          (else
            (bind _returnvalue_2 (`self.GetTransform` _asvehicle_blueprint))
            (bind _returnvalue_3 (`|SpawnActorFromClass` _weaponclass _returnvalue_2 "AlwaysSpawn" "OverrideRootScale" null null))
            (bind _mesh (`WheeledVehicle.Mesh` _asvehicle_blueprint))
            (`self.K2_AttachToComponent` _returnvalue_3 _mesh "SecondGunMount" "SnapToTarget" "SnapToTarget" "SnapToTarget" true)
            (set `/Game/VehicleAdvBP/Blueprints/VehicleBlueprint.SecondaryWeapon` _returnvalue_3 _asvehicle_blueprint)
            (`KismetSystemLibrary.PrintString` "Seocndary Added")))))
    (elif (== (`GameplayStatics.GetObjectClass` _secondaryweapon) (`self.WeaponClass`))
      (set `/Game/VehicleAdvBP/Blueprints/BP_BaseWeapon.CurrentAmmo` _returnvalue _secondaryweapon)
      (else
        (bind _returnvalue_4 (`|SpawnActorFromClass` _weaponclass _returnvalue_2 "AlwaysSpawn" "OverrideRootScale" null null))
        (`self.K2_AttachToComponent` _returnvalue_4 _mesh "GunMount" "SnapToTarget" "SnapToTarget" "SnapToTarget" true)
        (set `/Game/VehicleAdvBP/Blueprints/VehicleBlueprint.CurrentWeapon` _returnvalue_4 _asvehicle_blueprint)
        (`KismetSystemLibrary.PrintString` "Primary Added")))))

(event `self.ReceiveTick`
  (params (DeltaSeconds :type "Float (single-precision)"))
  ;[1 1 1] Pickup Movement
)

(fn `UserConstructionScript`)