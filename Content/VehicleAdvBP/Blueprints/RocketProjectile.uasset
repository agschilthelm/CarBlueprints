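; Rocket projectile Blueprint that trails smoke from its Propulsion socket and explodes on overlapping actors, ignoring the vehicle that fired it.
; Each valid overlap applies radial damage with falloff, using a full-damage inner radius at a third of the explosion radius, then calls OnExplode.
; A DoOnce limits the explosion to one radial impulse, sound and particle effect, then disables collision, hides the rocket and sets a short lifespan.
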(event `self.ReceiveBeginPlay`
  ;[1 1 1] Spawn Smoke Trail
  (`parent.ReceiveBeginPlay`)
  (`GameplayStatics.SpawnEmitterAttached` "/Game/Effects/P_SmokeTrail.P_SmokeTrail" (`self.ProjectileMesh`) "Propulsion"))

(event `self.ReceiveActorBeginOverlap`
  (params (OtherActor :type "Actor Object Reference"))
  (bind _explosionradius (`self.ExplosionRadius`))
  ;[1 1 1] Handle collison with object
  (bind _aswheeled_vehicle (cast `WheeledVehicle` OtherActor)
    (:`then`
      (if (!= _aswheeled_vehicle (`self.OwningVehicle`))
        (`GameplayStatics.ApplyRadialDamageWithFalloff` :`BaseDamage` (`self.Damage`) :`Origin` (`self.K2_GetActorLocation`) :`DamageInnerRadius` (/ _explosionradius 3.0) :`DamageOuterRadius` _explosionradius :`DamageFalloff` 2.0 :`DamageTypeClass` "/Script/Engine.DamageType" :`DamageCauser` self :`InstigatedByController` (`self.GetInstigatorController`) :!label _label)
        (`self.OnExplode`)))
    (:`CastFailed`
      (goto _label))))

(event `OnExplode`
  (bind _returnvalue (`self.K2_GetActorLocation`))
  ;[1 1 1] Execute when exploding
  (`/Engine/EditorBlueprintResources/StandardMacros.DoOnce` false
    (:`Completed`
      (`RadialForceComponent.FireImpulse` (`self.RadialForce`))
      (`GameplayStatics.PlaySoundAtLocation` "/Game/StarterContent/Audio/Explosion01.Explosion01" _returnvalue)
      (`GameplayStatics.SpawnEmitterAtLocation` (`self.OnDestroyEffect`) _returnvalue)
      (`self.SetActorEnableCollision` false)
      (`self.SetActorHiddenInGame` true)
      (`self.SetLifeSpan` 1.0))))

(event `self.ReceiveTick`
  (params (DeltaSeconds :type "Float (single-precision)"))
  (`parent.ReceiveTick` DeltaSeconds))

(fn `UserConstructionScript`
  (`parent.UserConstructionScript`))