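; BP_Projectile is a projectile actor that damages wheeled vehicles it overlaps, ignoring its owning vehicle.
; Overlaps cast to WheeledVehicle, then HandleHit applies the configured damage and damage type, crediting the instigator controller.
; Blocking hits only print a debug string and destroy the projectile without dealing damage.
; HandleDestroy simply destroys the actor and is called both inside HandleHit and again after it on overlap.
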(event `self.ReceiveHit`
  (params (MyComp :type "PrimitiveComponent Object Reference") (Other :type "Actor Object Reference") (OtherComp :type "PrimitiveComponent Object Reference") (bSelfMoved :type Boolean) (HitLocation :type "Vector Structure") (HitNormal :type "Vector Structure") (NormalImpulse :type "Vector Structure") (Hit :type "HitResult Structure (by ref)"))
  (`KismetSystemLibrary.PrintString` "HIT BLOCK")
  (`self.HandleDestroy`))

(event `self.ReceiveActorBeginOverlap`
  (params (OtherActor :type "Actor Object Reference"))
  (bind _aswheeled_vehicle (cast `WheeledVehicle` OtherActor))
  (if (!= _aswheeled_vehicle (`self.OwningVehicle`))
    (`self.HandleHit` _aswheeled_vehicle)
    (`self.HandleDestroy`)))

(fn `HandleDestroy`
  (`self.K2_DestroyActor`))

(fn `HandleHit`
  (params (DamagedActor :type "Actor Object Reference"))
  (`GameplayStatics.ApplyDamage` DamagedActor (`self.Damage`) (`self.GetInstigatorController`) self "/Script/Engine.DamageType")
  (`self.HandleDestroy`))

(fn `UserConstructionScript`)