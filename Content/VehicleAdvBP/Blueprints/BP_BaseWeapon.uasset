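; BP_BaseWeapon is a base weapon actor for a vehicle that fires BP_Projectile while ammo remains.
; Fire spends one round and line-traces from the passed camera along its forward vector, ignoring the owning vehicle.
; The projectile spawns at the weapon's location, rotated toward the impact point on a hit or along the camera's rotation otherwise.
; The event graph and construction script hold no active logic.
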(fn `Fire`
  (params (Camera :type "CameraComponent Object Reference"))
  (bind _returnvalue (`SceneComponent.K2_GetComponentLocation` Camera))
  (bind _returnvalue_2 (`self.K2_GetActorLocation`))
  (bind _currentammo (`self.CurrentAmmo`))
  (if (> _currentammo 0)
    (set `self.CurrentAmmo` (- _currentammo 1))
    (bind (_outhit _returnvalue_3) (`KismetSystemLibrary.LineTraceSingle` _returnvalue (+ _returnvalue (* (`KismetMathLibrary.GetForwardVector` (`SceneComponent.K2_GetComponentRotation` Camera)) (`self.MaxTraceRange`))) "TraceTypeQuery1" false (`|MakeArray` (`self.OwningVehicle`) :!type "Actor Object Reference")))
    (if _returnvalue_3
      (`|SpawnActorFromClass` "/Game/VehicleAdvBP/Blueprints/BP_Projectile.BP_Projectile_C" (`KismetMathLibrary.MakeTransform` _returnvalue_2 (`KismetMathLibrary.FindLookAtRotation` _returnvalue_2 (`.ImpactPoint` (`GameplayStatics.BreakHitResult` _outhit)))) "AlwaysSpawn" "OverrideRootScale" self null)
      (else
        (`|SpawnActorFromClass` "/Game/VehicleAdvBP/Blueprints/BP_Projectile.BP_Projectile_C" (`KismetMathLibrary.MakeTransform` _returnvalue_2 (`SceneComponent.K2_GetComponentRotation` Camera)) "AlwaysSpawn" "OverrideRootScale" self null)))))

(fn `UserConstructionScript`)